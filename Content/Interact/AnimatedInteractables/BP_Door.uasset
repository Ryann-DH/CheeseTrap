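; BP_Door is an interactable door that swings open when IsUnlocked is true, then closes itself after a short delay.
; A dot product between the door's forward vector and the direction to the player picks the swing direction.
; A timeline rotates the Arrow component, reversing once the forward play finishes.
; A FlipFlop with only A wired ignores every second interaction, and construction tints the Cube with PickupColor through a dynamic material.
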(event `/Game/Interfaces/Interface_Interact.INT_Interact`
  (params (PlayerRef :type "/Game/Player/BP_PlayerChar Object Reference"))
  (if (`self.IsUnlocked`)
    (`/Engine/EditorBlueprintResources/StandardMacros.FlipFlop`
      (:`A`
        (bind _returnvalue (`self.NewFunction` PlayerRef))
        (bind (_direction _alpha) (`Timeline|Timeline_0` :!label _label)
          (:`Update`
            (`SceneComponent.K2_SetRelativeRotation` (`self.Arrow`) (`KismetMathLibrary.MakeRotator` 0.0 0.0 (`KismetMathLibrary.Lerp` 0.0 _returnvalue _alpha)) false false))
          (:`Finished`
            (if (`|EnumEquality` _direction "Forward")
              (`KismetSystemLibrary.Delay` 1.0)
              (`self.reverse door`))))))))

(event `reverse door`
  (goto _label :!via `Reverse`))

(fn `NewFunction`
  (params (self2 :type "Actor Object Reference"))
  (returns (ReturnValue :type "Float (double-precision)"))
  (return (select `bool` (> (`KismetMathLibrary.Dot_VectorVector` (`KismetMathLibrary.GetDirectionUnitVector` (`self.K2_GetActorLocation`) (`self.K2_GetActorLocation` self2)) (`self.GetActorForwardVector`)) 0.0) :`false` -90.0 :`true` 90.0)))

(fn `UserConstructionScript`
  (bind _returnvalue (`PrimitiveComponent.CreateDynamicMaterialInstance` (`self.Cube`) 0 "/Game/Material/MAT_Color1.MAT_Color1" "None"))
  (bind _output_get (set `self.ColorDMI` _returnvalue))
  (`MaterialInstanceDynamic.SetVectorParameterValue` _output_get "Color" (`self.PickupColor`)))