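; BP_ElecCrod is an animated electric cord prop that shows power by moving a colored Cube along its local X axis.
; A looping timer from BeginPlay calls CordPowered, which plays the Alpha timeline to lerp the Cube between two fixed positions.
; StopTimeline clears that timer without stopping a timeline already in progress.
; The construction script creates a dynamic material instance tinted with CordColor.
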(event `CordPowered`
  (bind (_direction _alpha) (`Timeline|Alpha`)
    (:`Update`
      (`SceneComponent.K2_SetRelativeLocation` (`self.Cube`) (`KismetMathLibrary.MakeVector` (`KismetMathLibrary.Lerp` 1640.0 -1670.0 _alpha)) false false))))

(event `StopTimeline`
  (`KismetSystemLibrary.K2_ClearTimer` null "CordPowered"))

(event `self.ReceiveBeginPlay`
  (set `self.IsOff?` false)
  (if (not (`self.IsOff?`))
    (`KismetSystemLibrary.K2_SetTimer` null "CordPowered" 5.0 true)))

(fn `UserConstructionScript`
  (bind _returnvalue (`PrimitiveComponent.CreateDynamicMaterialInstance` (`self.Cube`) 0 "/Game/Material/MAT_Color1.MAT_Color1" "None"))
  (bind _output_get (set `self.Color DMI` _returnvalue))
  (`MaterialInstanceDynamic.SetVectorParameterValue` _output_get "Color" (`self.Cord Color`)))