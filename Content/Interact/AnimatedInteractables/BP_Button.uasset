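; BP_Button is a colour-keyed pressure button that opens a linked TargetCage when a BP_Pickup with a matching PickupColor overlaps it.
; A match sets the cage's IsOpen, then a timeline lowers the button mesh and flags it as pressed.
; The construction script tints the button to PickupColor through a dynamic material instance.
; Ending overlap never releases it, and older TargetDoor unlock logic remains disconnected.
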(event `self.Overlap.OnComponentEndOverlap`
  (params (OverlappedComponent :type "PrimitiveComponent Object Reference") (OtherActor :type "Actor Object Reference") (OtherComp :type "PrimitiveComponent Object Reference") (OtherBodyIndex :type Integer))
  (cast `/Game/Interact/Interactables/BP_Pickup` OtherActor))

(event `self.Overlap.OnComponentBeginOverlap`
  (params (OverlappedComponent :type "PrimitiveComponent Object Reference") (OtherActor :type "Actor Object Reference") (OtherComp :type "PrimitiveComponent Object Reference") (OtherBodyIndex :type Integer) (bFromSweep :type Boolean) (SweepResult :type "HitResult Structure (by ref)"))
  (bind _targetcage (`self.TargetCage`))
  (bind _asbp_pickup (cast `/Game/Interact/Interactables/BP_Pickup` OtherActor))
  (if (== (`/Game/Interact/Interactables/BP_Pickup.PickupColor` _asbp_pickup) (`self.PickupColor`))
    (`/Engine/EditorBlueprintResources/StandardMacros.IsValid` _targetcage
      (:`Is Valid`
        (set `/Game/Interact/Interactables/BP_Cage.IsOpen` true _targetcage)
        (bind (_direction _alphatrack) (`Timeline|Timeline`)
          (:`Update`
            (`SceneComponent.K2_SetRelativeLocation` (`self.Button`) (`KismetMathLibrary.MakeVector` 0.0 0.0 (`KismetMathLibrary.Lerp` 5.0 1.0 _alphatrack)) false false)
            (set `self.ButtonIsPressed?` true))))
      (:`Is Not Valid`
        (`KismetSystemLibrary.PrintString` "forgot to link door")))))

(fn `UserConstructionScript`
  (bind _returnvalue (`PrimitiveComponent.CreateDynamicMaterialInstance` (`self.Button`) 0 "/Game/Material/MAT_Color1.MAT_Color1" "None"))
  (bind _output_get (set `self.ColorDMI` _returnvalue))
  (`MaterialInstanceDynamic.SetVectorParameterValue` _output_get "Color" (`self.PickupColor`)))