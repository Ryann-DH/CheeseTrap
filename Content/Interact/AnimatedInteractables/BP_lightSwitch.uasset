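; Interactable light switch that is colour-coded to a power cord and acts on a linked target object.
; On interact it clears the target's "CordPowered" timer and plays a timeline that pitches the Arrow component to its flipped position, with no reverse path.
; The construction script tints the switch mesh with CordColor through a dynamic material instance.
; Disconnected cord-colour check and debug prints remain in the graph but never run.
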(event `/Game/Interfaces/Interface_Interact.INT_Interact`
  (params (PlayerRef :type "/Game/Player/BP_PlayerChar Object Reference"))
  (`KismetSystemLibrary.K2_ClearTimer` (`self.Target Object`) "CordPowered")
  (bind (_direction _alpha) (`Timeline|Alpha`)
    (:`Update`
      (`SceneComponent.K2_SetRelativeRotation` (`self.Arrow`) (`KismetMathLibrary.MakeRotator` 0.0 (`KismetMathLibrary.Lerp` 60.0 -30.0 _alpha)) false false))))

(fn `UserConstructionScript`
  (bind _returnvalue (`PrimitiveComponent.CreateDynamicMaterialInstance` (`self.switch`) 0 "/Game/Material/MAT_Color1.MAT_Color1" "None"))
  (bind _output_get (set `self.Color DMI` _returnvalue))
  (`MaterialInstanceDynamic.SetVectorParameterValue` _output_get "Color" (`self.Cord Color`)))