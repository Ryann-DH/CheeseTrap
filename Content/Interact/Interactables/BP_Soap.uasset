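; BP_Soap is an interactable pickup that works as an automatic soap-projectile weapon while the player holds it.
; INTInteract marks a free-handed player as holding, attaches Arrow to the player's Arrow2 and starts a looping FireAtEnemy timer.
; Each tick of that timer spawns BP_ProjectileSoap at ProjectileArrow's transform.
; INTDrop stops the timer, detaches the actor, restores SoapBar collision and physics, then attempts to clear the player's holding flag.
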(event `/Game/Interfaces/Interface_Interact.INT_Interact`
  (params (PlayerRef :type "/Game/Player/BP_PlayerChar Object Reference"))
  (bind _arrow (`self.Arrow`))
  (if (not (`/Game/Player/BP_PlayerChar.IsHolding` PlayerRef))
    (set `/Game/Player/BP_PlayerChar.IsHolding` true PlayerRef)
    (`PrimitiveComponent.SetSimulatePhysics` _arrow false)
    (`PrimitiveComponent.SetCollisionEnabled` _arrow "NoCollision")
    (`SceneComponent.K2_AttachToComponent` (`self.Arrow`) (`/Game/Player/BP_PlayerChar.Arrow2` PlayerRef) "None" "SnapToTarget" "KeepRelative" "KeepRelative" true)
    (`KismetSystemLibrary.K2_SetTimer` null "FireAtEnemy" 0.2 true)))

(event `FireAtEnemy`
  (`|SpawnActorFromClass` "/Game/Interact/Interactables/BP_ProjectileSoap.BP_ProjectileSoap_C" (`SceneComponent.K2_GetComponentToWorld` (`self.Projectile Arrow`)) "Undefined" "MultiplyWithRoot" null null))

(event `/Game/Interfaces/Interface_Interact.INT_Drop`
  (bind _soapbar (`self.SoapBar`))
  (`KismetSystemLibrary.K2_ClearTimer` null "FireAtEnemy")
  (`self.K2_DetachFromActor` "KeepWorld" "KeepWorld" "KeepWorld")
  (`PrimitiveComponent.SetCollisionEnabled` _soapbar "QueryAndPhysics")
  (`PrimitiveComponent.SetSimulatePhysics` _soapbar true)
  (bind _asbp_player_char (cast `/Game/Player/BP_PlayerChar` (`self.Target`)))
  (set `/Game/Player/BP_PlayerChar.IsHolding` false _asbp_player_char))

(fn `UserConstructionScript`)