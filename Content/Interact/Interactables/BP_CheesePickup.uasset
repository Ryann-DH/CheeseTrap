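; BP_CheesePickup is a cheese pickup that the player collects by walking into it.
; On BeginPlay, a timeline animates the Cube's relative height to move it vertically.
; When BP_PlayerChar overlaps the Box, it sets the player's HoldingCheese flag and destroys itself.
; The interact event is empty, and leftover unconnected nodes, including a BP_Hole cast, never run.
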(event `self.ReceiveBeginPlay`
  (bind (_direction _alpha) (`Timeline|Alpha` :`NewTime` 10.0)
    (:`Update`
      (`SceneComponent.K2_SetRelativeLocation` (`self.Cube`) (`KismetMathLibrary.MakeVector` 0.0 0.0 (`KismetMathLibrary.Lerp` 0.0 50.0 _alpha)) false false))))

(event `/Game/Interfaces/Interface_Interact.INT_Interact`
  (params (PlayerRef :type "/Game/Player/BP_PlayerChar Object Reference")))

(event `self.Box.OnComponentBeginOverlap`
  (params (OverlappedComponent :type "PrimitiveComponent Object Reference") (OtherActor :type "Actor Object Reference") (OtherComp :type "PrimitiveComponent Object Reference") (OtherBodyIndex :type Integer) (bFromSweep :type Boolean) (SweepResult :type "HitResult Structure (by ref)"))
  (bind _asbp_player_char (cast `/Game/Player/BP_PlayerChar` OtherActor))
  (set `/Game/Player/BP_PlayerChar.HoldingCheese?` true _asbp_player_char)
  (`self.K2_DestroyActor`))

(fn `UserConstructionScript`)