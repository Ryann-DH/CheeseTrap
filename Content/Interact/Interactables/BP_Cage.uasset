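; BP_Cage is an interactable cage actor that animates when the player interacts with it.
; On INTInteract, if IsOpen is true, a Timeline lerps the relative Z of the Arrow component upward.
; A helper, NewFunction, picks between the same two heights with a facing dot product, but nothing in this file calls it.
; IsOpen is never set here, and NewFunction0 is empty.
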(event `/Game/Interfaces/Interface_Interact.INT_Interact`
  (params (PlayerRef :type "/Game/Player/BP_PlayerChar Object Reference"))
  (if (`self.IsOpen`)
    (bind (_direction _alpha) (`Timeline|Timeline`)
      (:`Update`
        (`SceneComponent.K2_SetRelativeLocation` (`self.Arrow`) (`KismetMathLibrary.MakeVector` 0.0 0.0 (`KismetMathLibrary.Lerp` 50.0 160.0 _alpha)) false false)))))

(fn `NewFunction`
  (params (self2 :type "Actor Object Reference"))
  (returns (ReturnValue :type "Float (double-precision)"))
  (return (select `bool` (> (`KismetMathLibrary.Dot_VectorVector` (`KismetMathLibrary.GetDirectionUnitVector` (`self.K2_GetActorLocation`) (`self.K2_GetActorLocation`)) (`self.GetActorForwardVector`)) 0.0) :`false` 50.0 :`true` 160.0)))

(fn `NewFunction_0`)

(fn `UserConstructionScript`)