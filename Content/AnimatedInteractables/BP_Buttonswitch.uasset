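; Color-coded button switch whose construction script tints the Button mesh to PickupColor through a dynamic material instance.
; Its interaction logic is disconnected: the Box overlap and click events are empty, so the switch does nothing at runtime.
; The orphaned chain matches a BP_ElecCrod's color, sets TargetCord.IsOff and tilts the button with a timeline, or prints a warning if no target is linked.
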(event `self.Box.OnComponentBeginOverlap`
  (params (OverlappedComponent :type "PrimitiveComponent Object Reference") (OtherActor :type "Actor Object Reference") (OtherComp :type "PrimitiveComponent Object Reference") (OtherBodyIndex :type Integer) (bFromSweep :type Boolean) (SweepResult :type "HitResult Structure (by ref)")))

(event `self.Box.OnClicked`
  (params (TouchedComponent :type "PrimitiveComponent Object Reference") (ButtonPressed :type "Key Structure")))

(fn `NewFunction`)

(fn `UserConstructionScript`
  (bind _returnvalue (`PrimitiveComponent.CreateDynamicMaterialInstance` (`self.Button`) 0 "/Game/Material/MAT_Color1.MAT_Color1" "None"))
  (bind _output_get (set `self.ColorDMI` _returnvalue))
  (`MaterialInstanceDynamic.SetVectorParameterValue` _output_get "Color" (`self.PickupColor`)))