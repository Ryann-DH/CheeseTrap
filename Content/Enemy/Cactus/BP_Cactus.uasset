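; BP_Cactus is a stationary turret enemy that aims and fires BP_TurretProjectile from three spawn points while the player is inside its Box trigger.
; Overlap starts looping function-name timers: FollowPlayer1 turns three pivots toward the player, and three fire events spawn projectiles.
; End overlap clears the firing timers but not FollowPlayer1, so aiming continues.
; FollowPlayer is also timed, but has no definition here.
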(event `FireAtPlayer3`
  (`|SpawnActorFromClass` "/Game/Enemy/Turret/BP_TurretProjectile.BP_TurretProjectile_C" (`SceneComponent.K2_GetComponentToWorld` (`self.ArrowSpawn3`)) "Undefined" "MultiplyWithRoot" null null))

(event `FireAtPlayer1`
  (`|SpawnActorFromClass` "/Game/Enemy/Turret/BP_TurretProjectile.BP_TurretProjectile_C" (`SceneComponent.K2_GetComponentToWorld` (`self.Spawn2`)) "Undefined" "MultiplyWithRoot" null null))

(event `FollowPlayer1`
  (bind (_returnvalue_roll _returnvalue_pitch _returnvalue_yaw) (`KismetMathLibrary.BreakRotator` (`KismetMathLibrary.FindLookAtRotation` (`self.K2_GetActorLocation`) (`self.K2_GetActorLocation` (`GameplayStatics.GetPlayerCharacter` 0)))))
  (`SceneComponent.K2_SetWorldRotation` (`self.ArrowPivot1`) (`KismetMathLibrary.MakeRotator` _returnvalue_roll _returnvalue_pitch _returnvalue_yaw) false false)
  (`SceneComponent.K2_SetWorldRotation` (`self.PivotArm2`) (`KismetMathLibrary.MakeRotator` _returnvalue_roll _returnvalue_pitch _returnvalue_yaw) false false)
  (`SceneComponent.K2_SetWorldRotation` (`self.ArrowPivot3`) (`KismetMathLibrary.MakeRotator` _returnvalue_roll _returnvalue_pitch _returnvalue_yaw) false false))

(event `FireAtPlayer`
  (`|SpawnActorFromClass` "/Game/Enemy/Turret/BP_TurretProjectile.BP_TurretProjectile_C" (`SceneComponent.K2_GetComponentToWorld` (`self.ArrowSpawn1`)) "Undefined" "MultiplyWithRoot" null null))

(event `self.Box.OnComponentBeginOverlap`
  (params (OverlappedComponent :type "PrimitiveComponent Object Reference") (OtherActor :type "Actor Object Reference") (OtherComp :type "PrimitiveComponent Object Reference") (OtherBodyIndex :type Integer) (bFromSweep :type Boolean) (SweepResult :type "HitResult Structure (by ref)"))
  (cast `/Game/Player/BP_PlayerChar` OtherActor)
  (`KismetSystemLibrary.K2_SetTimer` null "FollowPlayer" 0.05 true)
  (`KismetSystemLibrary.K2_SetTimer` null "FollowPlayer1" 0.05 true)
  (`KismetSystemLibrary.K2_SetTimer` null "FireAtPlayer" 0.5 true)
  (`KismetSystemLibrary.K2_SetTimer` null "FireAtPlayer1" 0.5 true)
  (`KismetSystemLibrary.K2_SetTimer` null "FireAtPlayer3" 0.5 true))

(event `self.Box.OnComponentEndOverlap`
  (params (OverlappedComponent :type "PrimitiveComponent Object Reference") (OtherActor :type "Actor Object Reference") (OtherComp :type "PrimitiveComponent Object Reference") (OtherBodyIndex :type Integer))
  (cast `/Game/Player/BP_PlayerChar` OtherActor)
  (`KismetSystemLibrary.K2_ClearTimer` null "FollowPlayer")
  (`KismetSystemLibrary.K2_ClearTimer` null "FireAtPlayer")
  (`KismetSystemLibrary.K2_ClearTimer` null "FollowPlayer")
  (`KismetSystemLibrary.K2_ClearTimer` null "FireAtPlayer1")
  (`KismetSystemLibrary.K2_ClearTimer` null "FireAtPlayer3"))

(fn `UserConstructionScript`)