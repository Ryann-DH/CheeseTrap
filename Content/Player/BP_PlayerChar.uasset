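; Player character Blueprint with Enhanced Input movement, look and jump, plus object interaction, a score and health.
; Interact line-traces from the camera and sends an interface interact message to the hit actor, or a drop message to the stored actor while holding.
; Score and damage events update their totals with debug prints, and negative health quits the game.
; Push/pull input only prints its direction, and DropObject is an empty stub.
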(event `self.ReceiveBeginPlay`)

(event `EnhancedInput|/Game/Inputs/Input_Interact`
  (params (ActionValue :type Boolean) (ElapsedSeconds :type "Float (double-precision)") (TriggeredSeconds :type "Float (double-precision)") (InputAction :type "InputAction Object Reference" :default "/Game/Inputs/Input_Interact.Input_Interact"))
  (bind _camera (`self.Camera`))
  (bind _returnvalue (`SceneComponent.K2_GetComponentLocation` _camera))
  ;[0.03188 0.15 0.05229 0.5] INTERACT
  (:`Started`
    (if (`self.IsHolding`)
      (message `/Game/Interfaces/Interface_Interact.INT_Drop` (`self.HITObject`))
      (set `self.IsHolding` false)
      (else
        (bind (_outhit _returnvalue_2) (`KismetSystemLibrary.LineTraceSingle` :`Start` _returnvalue :`End` (+ _returnvalue (* (`SceneComponent.GetForwardVector` _camera) 800.0)) :`TraceChannel` "TraceTypeQuery1" :`DrawDebugType` "ForDuration"))
        (if _returnvalue_2
          (bind (_bblockinghit _binitialoverlap _time _distance _location _impactpoint _normal _impactnormal _physmat _hitactor) (`GameplayStatics.BreakHitResult` _outhit))
          (set `self.HITObject` _hitactor)
          (message `/Game/Interfaces/Interface_Interact.INT_Interact` _hitactor self))))))

(event `EnhancedInput|/Game/Inputs/Input_Movement`
  (params (ActionValue :type "Vector2D Structure") (ElapsedSeconds :type "Float (double-precision)") (TriggeredSeconds :type "Float (double-precision)") (InputAction :type "InputAction Object Reference" :default "/Game/Inputs/Input_Movement.Input_Movement"))
  (bind (_returnvalue_roll _returnvalue_pitch _returnvalue_yaw) (`KismetMathLibrary.BreakRotator` (`self.GetControlRotation`)))
  ; Char Movement
  ;;[0.1389 0.06429 0.15 0.5] Movement
  (:`Triggered`
    (`self.AddMovementInput` (`KismetMathLibrary.GetRightVector` (`KismetMathLibrary.MakeRotator` _returnvalue_roll 0.0 _returnvalue_yaw)) ActionValue_X)
    (`self.AddMovementInput` (`KismetMathLibrary.GetForwardVector` (`KismetMathLibrary.MakeRotator` 0.0 0.0 _returnvalue_yaw)) ActionValue_Y)))

(event `AddScore`
  (params (`Add Amount` :type Integer))
  ;[0.000285 0.01943 0.15 0.5] Score
  (bind _output_get (set `self.Score` (+ `Add Amount` (`self.Score`))))
  (`KismetSystemLibrary.PrintString` (`KismetStringLibrary.Conv_IntToString` _output_get)))

(event `EnhancedInput|/Game/Inputs/Input_Look`
  (params (ActionValue :type "Vector2D Structure") (ElapsedSeconds :type "Float (double-precision)") (TriggeredSeconds :type "Float (double-precision)") (InputAction :type "InputAction Object Reference" :default "/Game/Inputs/Input_Look.Input_Look"))
  ; Char Movement
  ;;[0.07591 0.07808 0.15 0.5] Look
  (:`Triggered`
    (`self.AddControllerYawInput` ActionValue_X)
    (`self.AddControllerPitchInput` ActionValue_Y)))

(event `EnhancedInput|/Game/Inputs/Input_Jump`
  (params (ActionValue :type Boolean) (ElapsedSeconds :type "Float (double-precision)") (TriggeredSeconds :type "Float (double-precision)") (InputAction :type "InputAction Object Reference" :default "/Game/Inputs/Input_Jump.Input_Jump"))
  ; Char Movement
  ;;[0.15 0.0705 0.0705 0.5] Jumpping
  (:`Started`
    (`self.Jump`))
  (:`Canceled`
    (`self.StopJumping`)))

(event `self.ReceiveAnyDamage`
  (params (Damage :type "Float (single-precision)") (DamageType :type "DamageType Object Reference") (InstigatedBy :type "Controller Object Reference") (DamageCauser :type "Actor Object Reference"))
  (bind _output_get (set `self.Helth` (- (`self.Helth`) Damage)))
  (`KismetSystemLibrary.PrintString` (`KismetStringLibrary.Conv_DoubleToString` _output_get))
  (if (< (`self.Helth`) 0.0)
    (`KismetSystemLibrary.QuitGame` null "Quit")))

(event `DropObject`)

(event `EnhancedInput|/Game/Inputs/Input_PushPull`
  (params (ActionValue :type "Vector2D Structure") (ElapsedSeconds :type "Float (double-precision)") (TriggeredSeconds :type "Float (double-precision)") (InputAction :type "InputAction Object Reference" :default "/Game/Inputs/Input_PushPull.Input_PushPull"))
  (:`Started`
    (if (!= ActionValue_X 0.0)
      (`KismetSystemLibrary.PrintString` "Push")
      (elif (!= ActionValue_Y 0.0)
        (`KismetSystemLibrary.PrintString` "Pull")))))

(fn `UserConstructionScript`)